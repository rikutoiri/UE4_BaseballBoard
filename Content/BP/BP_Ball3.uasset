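; BP_Ball3 is a baseball projectile that destroys itself about six seconds after it starts ticking, via a Delay on Tick.
; Hitting any hit-result target (Hit, 2BaseHit, 3BaseHit, HomeRun, NoHit) destroys it immediately.
; Bat contact drops projectile bounciness to a low value after a short delay.
; Other impacts randomize bounciness while the bat found via GetActorOfClass has IsHitBall false.
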(event `self.ReceiveTick`
  (params (DeltaSeconds :type "Float (single-precision)"))
  (`KismetSystemLibrary.Delay` 6.0)
  (`self.K2_DestroyActor` :!label _label))

(event `self.Ball.OnComponentHit`
  (params (HitComponent :type "PrimitiveComponent Object Reference") (OtherActor :type "Actor Object Reference") (OtherComp :type "PrimitiveComponent Object Reference") (NormalImpulse :type "Vector Structure") (Hit :type "HitResult Structure (by ref)"))
  (cast `/Game/BP/2BaseHit` OtherActor
    (:`then`
      (goto _label))
    (:`CastFailed`
      (cast `/Game/BP/Hit` OtherActor
        (:`then`
          (goto _label))
        (:`CastFailed`
          (cast `/Game/BP/3BaseHit` OtherActor
            (:`then`
              (goto _label))
            (:`CastFailed`
              (cast `/Game/BP/HomeRun` OtherActor
                (:`then`
                  (goto _label))
                (:`CastFailed`
                  (cast `/Game/BP/NoHit` OtherActor
                    (:`then`
                      (goto _label))
                    (:`CastFailed`
                      (cast `/Game/BP/BP_Bat1` OtherActor
                        (:`then`
                          (`KismetSystemLibrary.Delay` 0.2)
                          (bind _output_get (set `self.ProjectileMovement` (`self.ProjectileMovement`)))
                          (set `ProjectileMovementComponent.Bounciness` 0.1 _output_get))
                        (:`CastFailed`
                          (bind _returnvalue (`GameplayStatics.GetActorOfClass` "/Game/BP/BP_Bat1.BP_Bat1_C"))
                          (if (not (`/Game/BP/BP_Bat1.IsHitBall` _returnvalue))
                            (set `ProjectileMovementComponent.Bounciness` (`KismetMathLibrary.RandomFloatInRange` 0.5 1.0) (`self.ProjectileMovement`))))))))))))))))

(fn `UserConstructionScript`)