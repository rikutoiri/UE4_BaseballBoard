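; BP_ChangeUp is a changeup pitch ball for a baseball game, with gravity switched on after a delay.
; Tick pushes the ball briefly until BP_Bat1 reports a hit, then releases its constraint, and also runs velocity-checked cleanup.
; Collisions with result zones destroy the ball, while bat and other impacts adjust bounciness.
; Cleanup re-enables the pitcher's throw and resets pitcher and CountBoard flags, all fetched through GetActorOfClass.
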(event `self.ReceiveBeginPlay`
  (`KismetSystemLibrary.Delay` 3.0)
  (`PrimitiveComponent.SetEnableGravity` (`self.Ball`) true))

(event `self.ReceiveTick`
  (params (DeltaSeconds :type "Float (single-precision)"))
  (bind _force_x (`self.Force X`))
  (bind _ball (`self.Ball`))
  (bind _returnvalue (`GameplayStatics.GetActorOfClass` "/Game/BP/BP_pitcher.BP_pitcher_C"))
  (set `/Game/BP/BP_pitcher.IsThrow` false _returnvalue)
  (bind _returnvalue_2 (`GameplayStatics.GetActorOfClass` "/Game/BP/BP_Bat1.BP_Bat1_C"))
  (if (`/Game/BP/BP_Bat1.IsHitBall` _returnvalue_2)
    (`PrimitiveComponent.SetEnableGravity` (`self.Ball`) true)
    (`PrimitiveComponent.AddForce` _ball (0.0 0.0 0.0) "None" true)
    (`KismetSystemLibrary.Delay` 0.2)
    (`PrimitiveComponent.SetConstraintMode` (`self.Ball`) "None")
    (else
      (`PrimitiveComponent.AddForce` _ball (`KismetMathLibrary.MakeVector` _force_x _force_x) "None" true)
      (`KismetSystemLibrary.Delay` 0.4)
      (set `self.Force X` 0.0)))
  (if (not (== 0.0 (`KismetMathLibrary.VSize` (`self.GetVelocity` (`ActorComponent.GetOwner` (`self.Ball`))))))
    (`KismetSystemLibrary.Delay` 10.0))
  (`self.K2_DestroyActor` :!label _label)
  (bind _returnvalue_3 (`GameplayStatics.GetActorOfClass` "/Game/BP/BP_pitcher.BP_pitcher_C"))
  (set `/Game/BP/BP_pitcher.IsThrow` true _returnvalue_3)
  (bind _returnvalue_4 (`GameplayStatics.GetActorOfClass` "/Game/BP/CountBoard.CountBoard_C"))
  (set `/Game/BP/CountBoard.NotBallflg` false _returnvalue_4)
  (bind _returnvalue_5 (`GameplayStatics.GetActorOfClass` "/Game/BP/BP_pitcher.BP_pitcher_C"))
  (set `/Game/BP/BP_pitcher.out_hit` false _returnvalue_5))

(event `self.Ball.OnComponentHit`
  (params (HitComponent :type "PrimitiveComponent Object Reference") (OtherActor :type "Actor Object Reference") (OtherComp :type "PrimitiveComponent Object Reference") (NormalImpulse :type "Vector Structure") (Hit :type "HitResult Structure (by ref)"))
  (bind _other_actor (`self.Other Actor`))
  (bind _other_actor_2 (`self.Other Actor`))
  (bind _other_actor_3 (`self.Other Actor`))
  (bind _output_get (set `self.Other Actor` OtherActor))
  (cast `/Game/BP/BP_OutFeilder` _other_actor_2
    (:`then`
      (`KismetSystemLibrary.Delay` 4.0 :!label _label_2))
    (:`CastFailed`
      (cast `/Game/BP/BP_InFielder` _other_actor_2
        (:`then`
          (goto _label_2))
        (:`CastFailed`
          (cast `/Game/BP/2BaseHit` _output_get
            (:`then`
              (goto _label))
            (:`CastFailed`
              (cast `/Game/BP/Hit` _other_actor_3
                (:`then`
                  (goto _label))
                (:`CastFailed`
                  (cast `/Game/BP/3BaseHit` _other_actor_3
                    (:`then`
                      (goto _label))
                    (:`CastFailed`
                      (cast `/Game/BP/HomeRun` _other_actor_3
                        (:`then`
                          (goto _label))
                        (:`CastFailed`
                          (cast `/Game/BP/NoHit` _other_actor
                            (:`then`
                              (goto _label))
                            (:`CastFailed`
                              (cast `/Game/BP/BP_Bat1` _other_actor
                                (:`then`
                                  (`KismetSystemLibrary.Delay` 0.2)
                                  (bind _output_get_2 (set `self.ProjectileMovement` (`self.ProjectileMovement`)))
                                  (set `ProjectileMovementComponent.Bounciness` 0.1 _output_get_2))
                                (:`CastFailed`
                                  (bind _returnvalue (`GameplayStatics.GetActorOfClass` "/Game/BP/BP_Bat1.BP_Bat1_C"))
                                  (if (not (`/Game/BP/BP_Bat1.IsHitBall` _returnvalue))
                                    (set `ProjectileMovementComponent.Bounciness` (`KismetMathLibrary.RandomFloatInRange` 0.5 1.0) (`self.ProjectileMovement`))))))))))))))))))))

(fn `UserConstructionScript`)