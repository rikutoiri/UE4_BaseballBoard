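; BP_Curve is a baseball pitch, by name a curveball, that applies two opposite X impulses at spawn and enables gravity shortly after.
; Tick holds BP_pitcher's IsThrow false, and a delayed timeout destroys the ball and re-enables throwing.
; Hit-result actors trigger that cleanup immediately, fielders after a delay.
; Bat contact lowers projectile bounciness, while other impacts randomise it until BP_Bat1 reports a hit.
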(event `self.ReceiveBeginPlay`
  (`PrimitiveComponent.AddImpulse` (`self.Ball`) (20000.0 0.0 0.0) "None" false)
  (`PrimitiveComponent.AddImpulse` (`self.Ball`) (-20000.0 0.0 0.0) "None" false)
  (`KismetSystemLibrary.Delay` 0.7)
  (`PrimitiveComponent.SetEnableGravity` (`self.Ball`) true))

(event `self.ReceiveTick`
  (params (DeltaSeconds :type "Float (single-precision)"))
  (bind _returnvalue (`GameplayStatics.GetActorOfClass` "/Game/BP/BP_pitcher.BP_pitcher_C"))
  (set `/Game/BP/BP_pitcher.IsThrow` false _returnvalue)
  (`KismetSystemLibrary.Delay` 6.0)
  (`self.K2_DestroyActor` :!label _label)
  (`KismetSystemLibrary.PrintString` "Hello")
  (bind _returnvalue_2 (`GameplayStatics.GetActorOfClass` "/Game/BP/BP_pitcher.BP_pitcher_C"))
  (set `/Game/BP/BP_pitcher.IsThrow` true _returnvalue_2))

(event `self.Ball.OnComponentHit`
  (params (HitComponent :type "PrimitiveComponent Object Reference") (OtherActor :type "Actor Object Reference") (OtherComp :type "PrimitiveComponent Object Reference") (NormalImpulse :type "Vector Structure") (Hit :type "HitResult Structure (by ref)"))
  (bind _other_actor (`self.Other Actor`))
  (bind _other_actor_2 (`self.Other Actor`))
  (bind _other_actor_3 (`self.Other Actor`))
  (set `self.Other Actor` OtherActor)
  (`KismetSystemLibrary.PrintString` "Hello")
  (cast `/Game/BP/BP_OutFeilder` _other_actor_2
    (:`then`
      (`KismetSystemLibrary.Delay` 4.0 :!label _label_2)
      (goto _label))
    (:`CastFailed`
      (cast `/Game/BP/BP_InFielder` _other_actor_2
        (:`then`
          (goto _label_2))
        (:`CastFailed`
          (cast `/Game/BP/2BaseHit` _other_actor_2
            (:`then`
              (goto _label))
            (:`CastFailed`
              (cast `/Game/BP/Hit` _other_actor_3
                (:`then`
                  (goto _label))
                (:`CastFailed`
                  (cast `/Game/BP/3BaseHit` _other_actor_3
                    (:`then`
                      (goto _label))
                    (:`CastFailed`
                      (cast `/Game/BP/HomeRun` _other_actor_3
                        (:`then`
                          (goto _label))
                        (:`CastFailed`
                          (cast `/Game/BP/NoHit` _other_actor
                            (:`then`
                              (goto _label))
                            (:`CastFailed`
                              (cast `/Game/BP/BP_Bat1` _other_actor
                                (:`then`
                                  (`KismetSystemLibrary.Delay` 0.2)
                                  (bind _output_get (set `self.ProjectileMovement` (`self.ProjectileMovement`)))
                                  (set `ProjectileMovementComponent.Bounciness` 0.1 _output_get))
                                (:`CastFailed`
                                  (bind _returnvalue (`GameplayStatics.GetActorOfClass` "/Game/BP/BP_Bat1.BP_Bat1_C"))
                                  (if (not (`/Game/BP/BP_Bat1.IsHitBall` _returnvalue))
                                    (set `ProjectileMovementComponent.Bounciness` (`KismetMathLibrary.RandomFloatInRange` 0.5 1.0) (`self.ProjectileMovement`))))))))))))))))))))

(fn `UserConstructionScript`)