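; Player-controlled bat for a two-player baseball game, taking input from whichever player's turn the ScoreBoard reports on each Tick.
; The Swing input drives timelines that rotate the bat through a swing and back, with the return started after a delay on release.
; MoveRight nudges the batter sideways in Tick within MovePower limits, and contact with BP_Ball3 sets IsHitBall.
; Construction Script sets the bat's starting rotation from Battype and mirrors its scale.
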(event `InputAction|Swing`
  (params (Key :type "Key Structure"))
  (bind _bat (`self.Bat`))
  (:`Pressed`
    ;[1 1 1] バットのスウィング
    (set `self.IsSwing` true)
    (bind (_direction _rotationz _tateburi) (`Timeline|Swing` :!label _label)
      (:`Update`
        (`SceneComponent.K2_SetRelativeRotation` _bat (`KismetMathLibrary.MakeRotator` 0.0 _tateburi _rotationz) false false))
      (:`Finished`
        (set `self.IsSwing` false)
        (bind (_direction_2 _furimodoshi _tate) (`Timeline|SwingReturn` :!via `SetNewTime` :!label _label_2)
          (:`Update`
            (`SceneComponent.K2_SetRelativeRotation` _bat (`KismetMathLibrary.MakeRotator` 0.0 _tate _furimodoshi) false false))
          (:`Finished`
            (goto _label :!via `SetNewTime`))))))
  (:`Released`
    (`KismetSystemLibrary.Delay` 1.0)
    (goto _label_2)))

(event `InputAxis|MoveRight`
  (params (AxisValue :type "Float (single-precision)"))
  (if (== AxisValue 0.0)
    (set `self.IsLeftKey` false)
    (set `self.IsRightKey` false)
    (elif (> 0.0 AxisValue)
      ;[1 1 1] バッターの移動処理が行えるか
      (set `self.IsLeftKey` true)
      (elif (< 0.0 AxisValue)
        (set `self.IsRightKey` true)))))

(event `self.ReceiveTick`
  (params (DeltaSeconds :type "Float (single-precision)"))
  (bind _returnvalue (`GameplayStatics.GetPlayerController` 1))
  (bind _returnvalue_2 (`GameplayStatics.GetPlayerController` 0))
  (bind _movepower (`self.MovePower`))
  (bind _movepower_2 (`self.MovePower`))
  (bind _returnvalue_3 (`GameplayStatics.GetActorOfClass` "/Game/BP/ScoreBoard.ScoreBoard_C"))
  (if (`/Game/BP/ScoreBoard.IsTurn1P` _returnvalue_3)
    (`self.EnableInput` _returnvalue_2)
    ;[1 1 1] バッターの移動
    (`self.DisableInput` _returnvalue)
    (else
      (`self.EnableInput` _returnvalue)
      (`self.DisableInput` _returnvalue_2)))
  (if (`self.IsLeftKey`)
    (if (< _movepower_2 5.0)
      (set `self.MovePower` (+ _movepower_2 1.0))
      (`self.K2_AddActorLocalOffset` (0.0 5.0 0.0)))
    (elif (`self.IsRightKey`)
      (if (> _movepower -5.0)
        (set `self.MovePower` (- _movepower 1.0))
        (`self.K2_AddActorLocalOffset` (0.0 -5.0 0.0))))))

(event `self.Cube.OnComponentHit`
  (params (HitComponent :type "PrimitiveComponent Object Reference") (OtherActor :type "Actor Object Reference") (OtherComp :type "PrimitiveComponent Object Reference") (NormalImpulse :type "Vector Structure") (Hit :type "HitResult Structure (by ref)"))
  (cast `/Game/BP/BP_Ball3` OtherActor) ; ボールとバットが当たったら
  (set `self.IsHitBall` true) ; IｓHitBallをTrueにする
)

(event `self.ReceiveBeginPlay`)

(fn `SwingBat`)

(fn `UserConstructionScript`
  (set `self.StartRotation` (select `byte` (`self.Battype`) :`0` (struct :`Yaw` 20.0) :`1` (struct) :!type "Rotator Structure"))
  (set `self.StartRotation` (select `byte` (`self.Battype`) :`0` (struct :`Yaw` -20.0) :`1` (struct) :!type "Rotator Structure"))
  (`SceneComponent.K2_SetRelativeRotation` (`self.Bat`) (`self.StartRotation`) false false)
  (switch `/Game/Mesh/BatType` (cast `/Game/Mesh/BatType` (`self.Battype`))
    (:`NewEnumerator0`
      (`SceneComponent.SetRelativeScale3D` (`self.Bat`) (-1.0 1.0 1.0)))))