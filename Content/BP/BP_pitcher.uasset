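; Player-controlled pitcher for a baseball game that sidesteps within a small range and throws balls at the batter.
; Tick hands input to one of two players based on the ScoreBoard turn and advances the throw cooldown.
; Pulling the ThrowVertical stick stretches a spring; snapping it back spawns a straight, change-up, shuuto or curve ball per held button and resets bat hit flags.
; A plain throw action and debug aim rotation are also bound.
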(event `Key|Left`
  (params (Key :type "Key Structure"))
  ;[1 1 1] ピッチャーの移動
  (:`Pressed`
    (set `self.IsLeftKey` true))
  (:`Released`
    (set `self.IsLeftKey` false)))

(event `Key|Gamepad_RightTrigger`
  (params (Key :type "Key Structure"))
  ;[1 1 1] デバッグ用投げる向きの変更
  (:`Pressed`
    (`self.K2_AddActorLocalRotation` (`KismetMathLibrary.MakeRotator` 0.0 0.0 (+ 0.0 -10.0)) :!label _label)))

(event `InputAxis|TurnRate`
  (params (AxisValue :type "Float (single-precision)"))
  ;[1 1 1] ピッチャーの移動
  (if (== AxisValue 0.0)
    (set `self.IsRightKey` false)
    (set `self.IsLeftKey` false)
    (elif (> AxisValue 0.0)
      (set `self.IsRightKey` true)
      (elif (< AxisValue 0.0)
        (set `self.IsLeftKey` true)))))

(event `Key|F`
  (params (Key :type "Key Structure"))
  ;[1 1 1] デバッグ用投げる向きの変更
  (:`Pressed`
    (goto _label)))

(event `Key|Right`
  (params (Key :type "Key Structure"))
  ;[1 1 1] ピッチャーの移動
  (:`Pressed`
    (set `self.IsRightKey` true))
  (:`Released`
    (set `self.IsRightKey` false)))

(event `Key|G`
  (params (Key :type "Key Structure"))
  ;[1 1 1] デバッグ用投げる向きの変更
  (:`Pressed`
    (`self.K2_AddActorLocalRotation` (`KismetMathLibrary.MakeRotator` 0.0 0.0 (+ 0.0 10.0)) :!label _label_2)))

(event `Key|Gamepad_LeftTrigger`
  (params (Key :type "Key Structure"))
  ;[1 1 1] デバッグ用投げる向きの変更
  (:`Pressed`
    (goto _label_2)))

(event `self.ReceiveTick`
  (params (DeltaSeconds :type "Float (single-precision)"))
  (bind _returnvalue (`GameplayStatics.GetPlayerController` 1))
  (bind _returnvalue_2 (`GameplayStatics.GetPlayerController` 0))
  (bind _returnvalue_3 (`GameplayStatics.GetPlayerController` 1))
  (bind _returnvalue_4 (`GameplayStatics.GetPlayerController` 0))
  (bind _movepower (`self.MovePower`))
  (bind _movepower_2 (`self.MovePower`))
  (bind _asgame_instance_ai (cast `/Game/BP/GameInstance_AI` (`GameplayStatics.GetGameInstance`)))
  (switch `int` (`/Game/BP/GameInstance_AI.Game_AI` _asgame_instance_ai)
    (:`0`
      (bind _returnvalue_5 (`GameplayStatics.GetActorOfClass` "/Game/BP/ScoreBoard.ScoreBoard_C"))
      (if (`/Game/BP/ScoreBoard.IsTurn1P` _returnvalue_5)
        (`self.DisableInput` _returnvalue_2)
        (`self.EnableInput` _returnvalue)
        (else
          (`self.DisableInput` _returnvalue)
          (`self.EnableInput` _returnvalue_2))))
    (:`1`
      ;[1 1 1] プレイヤー切り替え
      (bind _returnvalue_6 (`GameplayStatics.GetActorOfClass` "/Game/BP/ScoreBoard.ScoreBoard_C"))
      (if (`/Game/BP/ScoreBoard.IsTurn1P` _returnvalue_6)
        (`self.DisableInput` _returnvalue_4)
        (`self.EnableInput` _returnvalue_3)
        (else
          (`self.DisableInput` _returnvalue_3)
          (`self.EnableInput` _returnvalue_4)))))
  (if (> (`self.ThrowTime`) (`self.IsThrowCnt`))
    (set `self.IsThrowCnt` (+ (`self.IsThrowCnt`) 1)))
  ;[1 1 1] ピッチャーの移動に必要な処理
  (if (`self.IsLeftKey`)
    (if (< _movepower_2 5.0)
      (set `self.MovePower` (+ _movepower_2 1.0))
      (`self.K2_AddActorLocalOffset` (0.0 3.0 0.0)))
    (elif (`self.IsRightKey`)
      (if (> _movepower -5.0)
        (set `self.MovePower` (- _movepower 1.0))
        (`self.K2_AddActorLocalOffset` (0.0 -3.0 0.0))))))

(event `InputAxis|ThrowVertical`
  (params (AxisValue :type "Float (single-precision)"))
  (bind _arrow (`self.Arrow`))
  (bind _fakeball (`self.FakeBall`))
  (bind _returnvalue (`SceneComponent.K2_GetComponentLocation` _arrow))
  (bind _returnvalue_2 (`SceneComponent.K2_GetComponentRotation` _arrow))
  (bind _output_get (set `self.Axis Value` AxisValue))
  (if (> 0.1 _output_get)
    (if (`self.IsThrow`)
      (`SceneComponent.SetVisibility` _fakeball true false)
      (`SceneComponent.K2_SetRelativeTransform` (`self.Spring`) (`KismetMathLibrary.MakeTransform` (-178.0 0.0 -43.0) (struct) (`KismetMathLibrary.MakeVector` (+ 1.25 (`self.Axis Value`)) 0.8 0.8)) false false)
      (`SceneComponent.K2_SetRelativeTransform` (`self.CSGMesh_C309617D`) (`KismetMathLibrary.MakeTransform` (`KismetMathLibrary.MakeVector` (+ 166.999832 (* (`self.Axis Value`) 200.0)) -5.000829 -48.0) (struct :`Yaw` 180.0) (1.25 1.25 1.25)) false false)
      (if (< (`self.Axis Value`) (`self.Power`))
        (set `self.Power` (`self.Axis Value`))
        (elif (> (- (`KismetMathLibrary.Abs` (`self.Power`)) (`KismetMathLibrary.Abs` (`self.Axis Value`))) 0.95)
          (set `self.Power` (`self.Axis Value`))
          (bind _returnvalue_3 (`GameplayStatics.GetActorOfClass` "/Game/BP/Hit.Hit_C"))
          ;[1 1 1] ボールを投げるスティック
          (if (`/Game/BP/Hit.RunTurn` _returnvalue_3)
            _
            (elif (`self.IsThrow`)
              (if (== (`self.IsThrowCnt`) 120)
                (`GameplayStatics.PlaySoundAtLocation` "/Game/Sounds/nageru.nageru" (371.0 -803.0 6.0) (struct) 1.0 1.0 0.0 null null null)
                (if (`self.ChangeUpFlg`)
                  (`|SpawnActorFromClass` "/Game/BP/BP_ChangeUp.BP_ChangeUp_C" (`KismetMathLibrary.MakeTransform` _returnvalue _returnvalue_2) "Undefined" "OverrideRootScale" null null)
                  (elif (`self.SyuhtoFlug`)
                    (`|SpawnActorFromClass` "/Game/BP/BP_Syuhto.BP_Syuhto_C" (`KismetMathLibrary.MakeTransform` _returnvalue _returnvalue_2) "Undefined" "OverrideRootScale" null null)
                    (elif (`self.CurveFlg`)
                      (`|SpawnActorFromClass` "/Game/BP/BP_Curve2.BP_Curve2_C" (`KismetMathLibrary.MakeTransform` _returnvalue _returnvalue_2) "Undefined" "OverrideRootScale" null null)
                      (else
                        (`|SpawnActorFromClass` "/Game/BP/BP_Ball3.BP_Ball3_C" (`KismetMathLibrary.MakeTransform` _returnvalue _returnvalue_2) "Undefined" "OverrideRootScale" null null)))))
                (bind _returnvalue_4 (`GameplayStatics.GetActorOfClass` "/Game/BP/BP_Bat1.BP_Bat1_C"))
                (set `/Game/BP/BP_Bat1.IsHitBall` false _returnvalue_4)
                (set `self.IsThrowCnt` 0)
                (set `/Game/BP/BP_Bat1.SwingStrike` false _returnvalue_4))))))
      (else
        (`SceneComponent.SetVisibility` _fakeball false false)))))

(event `InputAction|ChangeUp`
  (params (Key :type "Key Structure"))
  ;[1 1 1] Aボタン長押しでチェンジアップ
  (:`Pressed`
    (set `self.ChangeUpFlg` true))
  (:`Released`
    (set `self.ChangeUpFlg` false)))

(event `InputAction|throw`
  (params (Key :type "Key Structure"))
  (bind _arrow (`self.Arrow`))
  (:`Released`
    ;[1 1 1] ボール投げる
    (if (`self.IsThrow`)
      (if (== (`self.IsThrowCnt`) (`self.ThrowTime`))
        (`|SpawnActorFromClass` "/Game/BP/BP_Ball3.BP_Ball3_C" (`KismetMathLibrary.MakeTransform` (`SceneComponent.K2_GetComponentLocation` _arrow) (`SceneComponent.K2_GetComponentRotation` _arrow)) "Undefined" "OverrideRootScale" null null)
        (bind _returnvalue (`GameplayStatics.GetActorOfClass` "/Game/BP/BP_Bat1.BP_Bat1_C"))
        (set `/Game/BP/BP_Bat1.IsHitBall` false _returnvalue)
        (set `self.IsThrowCnt` 0)))))

(event `Key|Zero`
  (params (Key :type "Key Structure"))
  ;[1 1 1] ボール投げる
  (:`Pressed`
    (bind _returnvalue (`GameplayStatics.GetActorOfClass` "/Game/BP/BP_Bat1.BP_Bat1_C"))
    (set `/Game/BP/BP_Bat1.IsHitBall` false _returnvalue)))

(event `InputAction|Syuhto`
  (params (Key :type "Key Structure"))
  (:`Pressed`
    (set `self.SyuhtoFlug` true))
  (:`Released`
    (set `self.SyuhtoFlug` false)))

(event `InputAction|Curve`
  (params (Key :type "Key Structure"))
  (:`Pressed`
    (set `self.CurveFlg` true))
  (:`Released`
    (set `self.CurveFlg` false)))

(fn `UserConstructionScript`)