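; AI baseball pitcher that exists only when GameAI is 0, otherwise destroying itself on Tick.
; On 1P's turn, BP_pitcher's IsThrow winds AIthrow down, driving the spring's scale.
; At full wind-up, if its own IsThrow is set and no run is underway, it spawns a random change-up, shuuto, curve or class-less default and resets the bat's hit flag.
; Input flags go unread, and random sideways movement is disconnected.
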(event `Key|Left`
  (params (Key :type "Key Structure"))
  ;[1 1 1] ピッチャーの移動
  (:`Pressed`
    (set `self.IsLeftKey` true))
  (:`Released`
    (set `self.IsLeftKey` false)))

(event `Key|Right`
  (params (Key :type "Key Structure"))
  ;[1 1 1] ピッチャーの移動
  (:`Pressed`
    (set `self.IsRightKey` true))
  (:`Released`
    (set `self.IsRightKey` false)))

(event `self.ReceiveTick`
  (params (DeltaSeconds :type "Float (single-precision)"))
  (bind _arrow (`self.Arrow`))
  (bind _fakeball (`self.FakeBall`))
  (bind _returnvalue (`SceneComponent.K2_GetComponentLocation` _arrow))
  (bind _returnvalue_2 (`SceneComponent.K2_GetComponentRotation` _arrow))
  (bind _asgame_instance_ai (cast `/Game/BP/GameInstance_AI` (`GameplayStatics.GetGameInstance`)))
  (switch `int` (`/Game/BP/GameInstance_AI.Game_AI` _asgame_instance_ai)
    (:`Default`
      (`self.K2_DestroyActor` :!label _label))
    (:`0`
      ;[1 1 1] プレイヤー切り替え
      (bind _returnvalue_3 (`GameplayStatics.GetActorOfClass` "/Game/BP/ScoreBoard.ScoreBoard_C"))
      (if (`/Game/BP/ScoreBoard.IsTurn1P` _returnvalue_3)
        (bind _returnvalue_4 (`GameplayStatics.GetActorOfClass` "/Game/BP/BP_pitcher.BP_pitcher_C"))
        (if (`/Game/BP/BP_pitcher.IsThrow` _returnvalue_4)
          (if (> (`self.AIthrow`) -1.0)
            (set `self.AIthrow` (- (`self.AIthrow`) 0.01))
            (else
              (set `self.AIthrow` 0.0 :!label _label_2)))
          (else
            (goto _label_2)))
        (set `self.Axis Value` (`self.AIthrow`))
        (`SceneComponent.K2_SetRelativeTransform` (`self.Spring`) (`KismetMathLibrary.MakeTransform` (-178.0 0.0 -43.0) (struct) (`KismetMathLibrary.MakeVector` (+ 1.25 (`self.Axis Value`)) 0.8 0.8)) false false)
        (if (>= -1.0 (`self.AIthrow`))
          (if (`self.IsThrow`)
            (`SceneComponent.SetVisibility` _fakeball true false)
            (`SceneComponent.K2_SetRelativeTransform` (`self.CSGMesh_C309617D`) (`KismetMathLibrary.MakeTransform` (`KismetMathLibrary.MakeVector` (+ 166.999832 (* (`self.Axis Value`) 200.0)) -5.000829 -48.0) (struct :`Yaw` 180.0) (1.25 1.25 1.25)) false false)
            (set `self.RandomChange` (`KismetMathLibrary.RandomInteger` 6))
            (bind _returnvalue_5 (`GameplayStatics.GetActorOfClass` "/Game/BP/Hit.Hit_C"))
            ;[1 1 1] ボールを投げるスティック
            (if (`/Game/BP/Hit.RunTurn` _returnvalue_5)
              _
              (elif (`self.IsThrow`)
                (if (== (`self.IsThrowCnt`) 120)
                  _
                  (else
                    _))
                (switch `int` (`self.RandomChange`)
                  (:`0`
                    (`|SpawnActorFromClass` "/Game/BP/BP_ChangeUp.BP_ChangeUp_C" (`KismetMathLibrary.MakeTransform` _returnvalue _returnvalue_2) "Undefined" "OverrideRootScale" null null))
                  (:`1`
                    (`|SpawnActorFromClass` "/Game/BP/BP_Syuhto.BP_Syuhto_C" (`KismetMathLibrary.MakeTransform` _returnvalue _returnvalue_2) "Undefined" "OverrideRootScale" null null))
                  (:`2`
                    (`|SpawnActorFromClass` "/Game/BP/BP_Curve2.BP_Curve2_C" (`KismetMathLibrary.MakeTransform` _returnvalue _returnvalue_2) "Undefined" "OverrideRootScale" null null))
                  (:`3`
                    (`|SpawnActorFromClass` "/Game/BP/BP_Ball3.BP_Ball3_C" (`KismetMathLibrary.MakeTransform` _returnvalue _returnvalue_2) "Undefined" "OverrideRootScale" null null :!label _label_3))
                  (:`4`
                    (goto _label_3))
                  (:`5`
                    (goto _label_3)))
                (bind _returnvalue_6 (`GameplayStatics.GetActorOfClass` "/Game/BP/BP_Bat1.BP_Bat1_C"))
                (set `/Game/BP/BP_Bat1.IsHitBall` false _returnvalue_6)
                (set `self.IsThrowCnt` 0)))
            (else
              (`SceneComponent.SetVisibility` _fakeball false false))))))
    (:`1`
      (goto _label))))

(event `InputAction|ChangeUp`
  (params (Key :type "Key Structure"))
  ;[1 1 1] Aボタン長押しでチェンジアップ
  (:`Pressed`
    (set `self.ChangeUpFlg` true))
  (:`Released`
    (set `self.ChangeUpFlg` false)))

(event `InputAction|Syuhto`
  (params (Key :type "Key Structure"))
  (:`Pressed`
    (set `self.SyuhtoFlug` true))
  (:`Released`
    (set `self.SyuhtoFlug` false)))

(event `InputAction|Curve`
  (params (Key :type "Key Structure"))
  (:`Pressed`
    (set `self.CurveFlg` true))
  (:`Released`
    (set `self.CurveFlg` false)))

(fn `UserConstructionScript`)