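; BP_Bat is an input-driven bat actor that swings a Bat component about its yaw axis, apparently like a flipper.
; The Swing input plays a timeline that drives yaw, and releasing it reverses the timeline from the end.
; The construction script uses Battype to set the starting rotation and mirror the component scale.
; Flip and Flop events tween between end and start rotations, but their test sequence is disconnected.
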(event `InputAction|Swing`
  (params (Key :type "Key Structure"))
  (:`Pressed`
    (`KismetSystemLibrary.PrintString` "Swing")
    (bind (_direction _rotationz) (`Timeline|Swing` :!label _label)
      (:`Update`
        (`SceneComponent.K2_SetRelativeRotation` (`self.Bat`) (`KismetMathLibrary.MakeRotator` 0.0 0.0 _rotationz) false false))))
  (:`Released`
    (goto _label :!via `ReverseFromEnd`)))

(event `self.ReceiveTick`
  (params (DeltaSeconds :type "Float (single-precision)")))

(event `self.ReceiveBeginPlay`)

(event `Flip`
  (`KismetSystemLibrary.MoveComponentTo` (`self.Bat`) (0.0 0.0 0.0) (`self.EndRotation`) false false (`self.FlipTime`)))

(event `Flop`
  (`KismetSystemLibrary.MoveComponentTo` (`self.Bat`) (0.0 0.0 0.0) (`self.StartRotation`) false false (`self.FlipTime`)))

(fn `UserConstructionScript`
  (set `self.StartRotation` (select `byte` (`self.Battype`) :`0` (struct :`Yaw` 20.0) :`1` (struct) :!type "Rotator Structure"))
  (set `self.StartRotation` (select `byte` (`self.Battype`) :`0` (struct :`Yaw` -20.0) :`1` (struct) :!type "Rotator Structure"))
  (`SceneComponent.K2_SetRelativeRotation` (`self.Bat`) (`self.StartRotation`) false false)
  (switch `/Game/Mesh/BatType` (cast `/Game/Mesh/BatType` (`self.Battype`))
    (:`NewEnumerator0`
      (`SceneComponent.SetRelativeScale3D` (`self.Bat`) (-1.0 1.0 1.0)))))