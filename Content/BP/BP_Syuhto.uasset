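; Baseball pitch actor, apparently the shuuto pitch, that launches its ball with an impulse on BeginPlay and enables gravity a second later.
; Tick applies a ForceX acceleration until a delay zeroes it, or releases the ball's constraint once BP_Bat1 reports a hit.
; Delayed timeouts, low speed or hit-zone contacts spawn smoke, destroy the ball, re-arm BP_pitcher and reset pitcher and CountBoard flags.
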(event `self.ReceiveBeginPlay`
  (bind _returnvalue (`GameplayStatics.GetActorOfClass` "/Game/BP/BP_pitcher.BP_pitcher_C"))
  (set `self.bp_pitcher` _returnvalue)
  (`PrimitiveComponent.AddImpulse` (`self.Ball`) (-25000.0 0.0 0.0) "None" false)
  (`KismetSystemLibrary.Delay` 1.0)
  (`PrimitiveComponent.SetEnableGravity` (`self.Ball`) true))

(event `self.ReceiveTick`
  (params (DeltaSeconds :type "Float (single-precision)"))
  (bind _ball (`self.Ball`))
  (if (`/Game/BP/BP_pitcher.out_hit` (`self.bp_pitcher`))
    (`KismetSystemLibrary.Delay` 5.0)
    (else
      (bind _returnvalue (`GameplayStatics.GetActorOfClass` "/Game/BP/BP_Bat1.BP_Bat1_C"))
      (if (`/Game/BP/BP_Bat1.IsHitBall` _returnvalue)
        (`PrimitiveComponent.AddForce` _ball (0.0 0.0 0.0) "None" true)
        (`KismetSystemLibrary.Delay` 0.2)
        (`PrimitiveComponent.SetConstraintMode` (`self.Ball`) "None")
        (else
          (`PrimitiveComponent.AddForce` _ball (`KismetMathLibrary.MakeVector` (`self.Force X`)) "None" true)
          (`KismetSystemLibrary.Delay` 0.6)
          (set `self.Force X` 0.0)))
      (if (not (> 10.0 (`KismetMathLibrary.VSize` (`self.GetVelocity` (`ActorComponent.GetOwner` (`self.Ball`))))))
        (`KismetSystemLibrary.Delay` 15.0))))
  (`GameplayStatics.SpawnEmitterAtLocation` "/Game/FX/Ball_smokeffect.Ball_smokeffect" (`SceneComponent.K2_GetComponentLocation` (`self.Ball`)) :!label _label)
  (`self.K2_DestroyActor`)
  (set `/Game/BP/BP_pitcher.IsThrow` true (`self.bp_pitcher`))
  (bind _returnvalue_2 (`GameplayStatics.GetActorOfClass` "/Game/BP/CountBoard.CountBoard_C"))
  (set `/Game/BP/CountBoard.NotBallflg` false _returnvalue_2)
  (set `/Game/BP/BP_pitcher.out_hit` false (`self.bp_pitcher`)))

(event `self.Ball.OnComponentHit`
  (params (HitComponent :type "PrimitiveComponent Object Reference") (OtherActor :type "Actor Object Reference") (OtherComp :type "PrimitiveComponent Object Reference") (NormalImpulse :type "Vector Structure") (Hit :type "HitResult Structure (by ref)"))
  (bind _other_actor (`self.Other Actor`))
  (bind _other_actor_2 (`self.Other Actor`))
  (set `self.Other Actor` OtherActor)
  (cast `/Game/BP/BP_OutFeilder` _other_actor
    (:`then`
      _)
    (:`CastFailed`
      (cast `/Game/BP/BP_InFielder` _other_actor
        (:`then`
          _)
        (:`CastFailed`
          (cast `/Game/BP/2BaseHit` _other_actor
            (:`then`
              (goto _label))
            (:`CastFailed`
              (cast `/Game/BP/Hit` _other_actor_2
                (:`then`
                  (goto _label))
                (:`CastFailed`
                  (cast `/Game/BP/3BaseHit` _other_actor_2
                    (:`then`
                      (goto _label))
                    (:`CastFailed`
                      (cast `/Game/BP/HomeRun` _other_actor_2
                        (:`then`
                          (goto _label))
                        (:`CastFailed`
                          (cast `/Game/BP/NoHit` (`self.Other Actor`))
                          (goto _label)))))))))))))
  (`KismetSystemLibrary.Delay` 4.0))

(fn `UserConstructionScript`)