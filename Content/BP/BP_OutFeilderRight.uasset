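; Right outfielder for a baseball game that moves along X on a timeline and catches batted balls for outs.
; Tick recolors its meshes blue or red from the ScoreBoard's turn.
; When one of four ball types enters its Sphere, it attaches the ball, flags BP_pitcher, updates CountBoard, calls CallCatchBallOutR and plays out sound, widget and material-scale effects.
; Box components show on catch and hide on end overlap.
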(event `self.ReceiveTick`
  (params (DeltaSeconds :type "Float (single-precision)"))
  (bind _cube (`self.Cube`))
  (bind _returnvalue (`GameplayStatics.GetActorOfClass` "/Game/BP/ScoreBoard.ScoreBoard_C"))
  (if (`/Game/BP/ScoreBoard.IsTurn1P` _returnvalue)
    (`PrimitiveComponent.SetMaterial` _cube 0 "/Game/Materials/FielderBlue.FielderBlue")
    (`PrimitiveComponent.SetMaterial` (`self.StaticMesh1`) 0 "/Game/Materials/FielderBlue.FielderBlue")
    (`PrimitiveComponent.SetMaterial` (`self.Cylinder`) 0 "/Game/Materials/FielderBlue.FielderBlue")
    (`PrimitiveComponent.SetMaterial` (`self.StaticMesh`) 0 "/Game/Materials/FielderBlue.FielderBlue")
    (`PrimitiveComponent.SetMaterial` (`self.Cylinder1`) 0 "/Game/Materials/FielderBlue.FielderBlue")
    (else
      (`PrimitiveComponent.SetMaterial` _cube 0 "/Game/Materials/FielderRed.FielderRed")
      (`PrimitiveComponent.SetMaterial` (`self.StaticMesh1`) 0 "/Game/Materials/FielderRed.FielderRed")
      (`PrimitiveComponent.SetMaterial` (`self.Cylinder`) 0 "/Game/Materials/FielderRed.FielderRed")
      (`PrimitiveComponent.SetMaterial` (`self.StaticMesh`) 0 "/Game/Materials/FielderRed.FielderRed")
      (`PrimitiveComponent.SetMaterial` (`self.Cylinder1`) 0 "/Game/Materials/FielderRed.FielderRed"))))

(event `self.ReceiveBeginPlay`
  (`SceneComponent.SetVisibility` (`self.Box1`) false false)
  (`SceneComponent.SetVisibility` (`self.Box2`) false false)
  (`SceneComponent.SetVisibility` (`self.Box3`) false false)
  (`SceneComponent.SetVisibility` (`self.Box`) false false)
  (set `self.DefaultLoacate` (`SceneComponent.K2_GetComponentLocation` (`self.OutFielder`)))
  (bind (_direction `_新規track_0`) (`Timeline|タイムライン_5`)
    (:`Update`
      (`self.K2_SetActorLocation` (+ (`self.DefaultLoacate`) (`KismetMathLibrary.MakeVector` (* `_新規track_0` 100.0)))))))

(event `self.Sphere.OnComponentBeginOverlap`
  (params (OverlappedComponent :type "PrimitiveComponent Object Reference") (OtherActor :type "Actor Object Reference") (OtherComp :type "PrimitiveComponent Object Reference") (OtherBodyIndex :type Integer) (bFromSweep :type Boolean) (SweepResult :type "HitResult Structure (by ref)"))
  (bind _returnvalue (`SceneComponent.K2_GetComponentLocation` (`self.Point`)))
  (bind _asbp_ball_3 (cast `/Game/BP/BP_Ball3` OtherActor)
    (:`then`
      (bind _output_get (set `self.As BP Ball 3` _asbp_ball_3))
      (`self.K2_SetActorLocation` _output_get _returnvalue false false)
      (`self.K2_AttachToComponent` (`self.As BP Ball 3`) (`self.Point`) "None" "KeepWorld" "KeepRelative" "KeepRelative" true) ; ボールを野手の子要素にする
    )
    (:`CastFailed`
      (bind _asbp_change_up (cast `/Game/BP/BP_ChangeUp` OtherActor)
        (:`then`
          (bind _output_get_2 (set `self.As BP Change Up` _asbp_change_up))
          (`self.K2_SetActorLocation` _output_get_2 _returnvalue false false)
          (`self.K2_AttachToComponent` (`self.As BP Change Up`) (`self.Point`) "None" "KeepWorld" "KeepRelative" "KeepRelative" true) ; ボールを野手の子要素にする
        )
        (:`CastFailed`
          (bind _asbp_syuhto (cast `/Game/BP/BP_Syuhto` OtherActor)
            (:`then`
              (bind _output_get_3 (set `self.As BP Syuhto` _asbp_syuhto))
              (`self.K2_SetActorLocation` _output_get_3 _returnvalue false false)
              (`self.K2_AttachToComponent` (`self.As BP Syuhto`) (`self.Point`) "None" "KeepWorld" "KeepRelative" "KeepRelative" true) ; ボールを野手の子要素にする
            )
            (:`CastFailed`
              (bind _asbp_curve_2 (cast `/Game/BP/BP_Curve2` OtherActor))
              (bind _output_get_4 (set `self.As BP Curve 2` _asbp_curve_2))
              (`self.K2_SetActorLocation` _output_get_4 _returnvalue false false)
              (`self.K2_AttachToComponent` (`self.As BP Curve 2`) (`self.Point`) "None" "KeepWorld" "KeepRelative" "KeepRelative" true) ; ボールを野手の子要素にする
            ))))))
  (bind _returnvalue_2 (`GameplayStatics.GetActorOfClass` "/Game/BP/BP_pitcher.BP_pitcher_C"))
  (set `/Game/BP/BP_pitcher.out_hit` true _returnvalue_2)
  (`SceneComponent.SetVisibility` (`self.Box1`) true false)
  (`SceneComponent.SetVisibility` (`self.Box2`) true false)
  (`SceneComponent.SetVisibility` (`self.Box3`) true false)
  (`SceneComponent.SetVisibility` (`self.Box`) true false)
  (bind _returnvalue_3 (`GameplayStatics.GetActorOfClass` "/Game/BP/CountBoard.CountBoard_C"))
  (set `/Game/BP/CountBoard.OutCount` (+ (`/Game/BP/CountBoard.OutCount` _returnvalue_3) 1) _returnvalue_3)
  (set `/Game/BP/CountBoard.StrikeCnt` 0 _returnvalue_3)
  (`self.CatchBallOutR`)
  (`GameplayStatics.PlaySound2D` "/Game/Sounds/アウト.アウト" 1.0 1.0 0.0 null null)
  (bind _returnvalue_4 (`|CreateWidget` "/Game/Widget/W_Out.W_Out_C"))
  (bind _output_get_5 (set `self.W_Out` _returnvalue_4))
  (`UserWidget.AddToViewport` _output_get_5 0)
  (bind (_direction `_新規track_0`) (`Timeline|タイムライン_1` :!via `PlayFromStart`)
    (:`Update`
      (`MeshComponent.SetScalarParameterValueOnMaterials` (`self.TestSphere`) "scale" `_新規track_0`))
    (:`Finished`
      (`Widget.RemoveFromParent` (`self.W_Out`)))))

(event `self.Sphere.OnComponentEndOverlap`
  (params (OverlappedComponent :type "PrimitiveComponent Object Reference") (OtherActor :type "Actor Object Reference") (OtherComp :type "PrimitiveComponent Object Reference") (OtherBodyIndex :type Integer))
  (cast `/Game/BP/BP_Ball3` OtherActor
    (:`then`
      _)
    (:`CastFailed`
      (cast `/Game/BP/BP_ChangeUp` OtherActor
        (:`then`
          _)
        (:`CastFailed`
          (cast `/Game/BP/BP_Syuhto` OtherActor
            (:`then`
              _)
            (:`CastFailed`
              (cast `/Game/BP/BP_Curve2` OtherActor)))))))
  (`SceneComponent.SetVisibility` (`self.Box1`) false false)
  (`SceneComponent.SetVisibility` (`self.Box2`) false false)
  (`SceneComponent.SetVisibility` (`self.Box3`) false false)
  (`SceneComponent.SetVisibility` (`self.Box`) false false)
  (bind _returnvalue (`GameplayStatics.GetActorOfClass` "/Game/BP/BP_pitcher.BP_pitcher_C"))
  (set `/Game/BP/BP_pitcher.out_hit` true _returnvalue)
  (`MeshComponent.SetScalarParameterValueOnMaterials` (`self.TestSphere`) "scale" 0.0))

(fn `UserConstructionScript`
  (`PrimitiveComponent.SetUseCCD` (`self.Box1`) true "None")
  (`PrimitiveComponent.SetUseCCD` (`self.Box`) true "None"))