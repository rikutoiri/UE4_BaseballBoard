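; AI batter for a baseball game that swings its bat when a BP_Ball3 enters its trigger box.
; Swing and SwingReturn timelines drive bat rotation, and construction sets bat rotation and scale from Battype.
; Bat and Cube hits by four ball classes set IsHitBall for foul handling.
; Tick toggles input around the ScoreBoard turn and applies limited sideways steps, though the logic setting the movement keys is disconnected.
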(event `self.Box.OnComponentBeginOverlap`
  (params (OverlappedComponent :type "PrimitiveComponent Object Reference") (OtherActor :type "Actor Object Reference") (OtherComp :type "PrimitiveComponent Object Reference") (OtherBodyIndex :type Integer) (bFromSweep :type Boolean) (SweepResult :type "HitResult Structure (by ref)"))
  (bind _bat (`self.Bat`))
  ;[1 1 1] バットのスウィング
  (cast `/Game/BP/BP_Ball3` OtherActor
    (:`then`
      (`KismetSystemLibrary.PrintString` "AI")
      (set `self.IsSwing` true)
      (bind (_direction _rotationz _tateburi) (`Timeline|Swing` :!label _label)
        (:`Update`
          (`SceneComponent.K2_SetRelativeRotation` _bat (`KismetMathLibrary.MakeRotator` 0.0 _tateburi _rotationz) false false))
        (:`Finished`
          (set `self.IsSwing` false)
          (bind (_direction_2 _furimodoshi _tate) (`Timeline|SwingReturn` :!via `SetNewTime` :!label _label_2)
            (:`Update`
              (`SceneComponent.K2_SetRelativeRotation` _bat (`KismetMathLibrary.MakeRotator` 0.0 _tate _furimodoshi) false false))
            (:`Finished`
              (goto _label :!via `SetNewTime`))))))
    (:`CastFailed`
      (`KismetSystemLibrary.Delay` 1.0)
      (goto _label_2))))

(event `self.ReceiveTick`
  (params (DeltaSeconds :type "Float (single-precision)"))
  (bind _movepower (`self.MovePower`))
  (bind _movepower_2 (`self.MovePower`))
  ;[1 1 1] プレイヤー切り替え
  (bind _returnvalue (`GameplayStatics.GetActorOfClass` "/Game/BP/ScoreBoard.ScoreBoard_C"))
  (if (`/Game/BP/ScoreBoard.IsTurn1P` _returnvalue)
    (`self.DisableInput` null)
    (`self.EnableInput` null)
    (else
      (`self.DisableInput` null)
      (`self.EnableInput` null)))
  ;[1 1 1] バッターの移動
  (if (`self.IsLeftKey`)
    (if (< _movepower_2 5.0)
      (set `self.MovePower` (+ _movepower_2 1.0))
      (`self.K2_AddActorLocalOffset` (0.0 5.0 0.0)))
    (elif (`self.IsRightKey`)
      (if (> _movepower -5.0)
        (set `self.MovePower` (- _movepower 1.0))
        (`self.K2_AddActorLocalOffset` (0.0 -5.0 0.0))))))

(event `self.Cube.OnComponentHit`
  (params (HitComponent :type "PrimitiveComponent Object Reference") (OtherActor :type "Actor Object Reference") (OtherComp :type "PrimitiveComponent Object Reference") (NormalImpulse :type "Vector Structure") (Hit :type "HitResult Structure (by ref)"))
  ;[1 1 1] ファールにするための処理
  (cast `/Game/BP/BP_Ball3` OtherActor ; ボールとバットが当たったら
    (:`then`
      _)
    (:`CastFailed`
      (cast `/Game/BP/BP_ChangeUp` OtherActor
        (:`then`
          _)
        (:`CastFailed`
          (cast `/Game/BP/BP_Syuhto` OtherActor
            (:`then`
              _)
            (:`CastFailed`
              (cast `/Game/BP/BP_Curve2` OtherActor)))))))
  (set `self.IsHitBall` true) ; IｓHitBallをTrueにする
)

(event `self.Bat.OnComponentHit`
  (params (HitComponent :type "PrimitiveComponent Object Reference") (OtherActor :type "Actor Object Reference") (OtherComp :type "PrimitiveComponent Object Reference") (NormalImpulse :type "Vector Structure") (Hit :type "HitResult Structure (by ref)"))
  (cast `/Game/BP/BP_Ball3` OtherActor ; ボールとバットが当たったら
    (:`then`
      _)
    (:`CastFailed`
      (cast `/Game/BP/BP_ChangeUp` OtherActor
        (:`then`
          _)
        (:`CastFailed`
          (cast `/Game/BP/BP_Syuhto` OtherActor
            (:`then`
              _)
            (:`CastFailed`
              (cast `/Game/BP/BP_Curve2` OtherActor)))))))
  (set `self.IsHitBall` true) ; IｓHitBallをTrueにする
)

(fn `SwingBat`)

(fn `UserConstructionScript`
  (set `self.StartRotation` (select `byte` (`self.Battype`) :`0` (struct :`Yaw` 20.0) :`1` (struct) :!type "Rotator Structure"))
  (set `self.StartRotation` (select `byte` (`self.Battype`) :`0` (struct :`Yaw` -20.0) :`1` (struct) :!type "Rotator Structure"))
  (`SceneComponent.K2_SetRelativeRotation` (`self.Bat`) (`self.StartRotation`) false false)
  (switch `/Game/Mesh/BatType` (cast `/Game/Mesh/BatType` (`self.Battype`))
    (:`NewEnumerator0`
      (`SceneComponent.SetRelativeScale3D` (`self.Bat`) (-1.0 1.0 1.0)))))